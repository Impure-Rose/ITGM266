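; Elevator actor that the player toggles between its base position and an upper or target floor with the Interact input.
; A Sphere overlap enables input for player 0 on entry and disables it on exit, so Interact works only nearby.
; Each press plays a sound and flips HasMoved, moving ElevatorTest over ElevatorMoveSpeed seconds to either Floor1's location or the zero relative location.
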(event OnComponentBeginOverlap(Sphere)
  (params (OverlappedComponent :type Primitive%20Component%20Object%20Reference) (OtherActor :type Actor%20Object%20Reference) (OtherComp :type Primitive%20Component%20Object%20Reference) (OtherBodyIndex :type Integer) (bFromSweep :type Boolean) (SweepResult :type Hit%20Result%20Structure%20%28by%20ref%29))
  (Input|EnableInput (Game|GetPlayerController 0)))

(event OnComponentEndOverlap(Sphere)
  (params (OverlappedComponent :type Primitive%20Component%20Object%20Reference) (OtherActor :type Actor%20Object%20Reference) (OtherComp :type Primitive%20Component%20Object%20Reference) (OtherBodyIndex :type Integer))
  (Input|DisableInput (Game|GetPlayerController 0)))

(event EventBeginPlay)

(event Collision|EventActorBeginOverlap
  (params (OtherActor :type Actor%20Object%20Reference)))

(event EventTick
  (params (DeltaSeconds :type Float%20%28single-precision%29)))

(event Input|ActionEvents|InputActionInteract
  (params (Key :type Key%20Structure :default "None"))
  (bind _elevatortest (Variables|Components|GetElevatorTest))
  (bind _elevatormovespeed (Variables|ElevatorSetup|GetElevatorMoveSpeed))
  (:Pressed
    (Audio|PlaySoundatLocation "/Game/FinalAssets/audio/ElevartorNew.ElevartorNew" (Transformation|GetWorldLocation (Variables|Components|GetElevatorTest)) "0, 0, 0" 1.0 1.0 0.0 0 0 0)
    (if (Variables|ElevatorSetup|GetHasMoved?)
      (Components|MoveComponentTo _elevatortest "0, 0, 0" "0, 0, 0" false false _elevatormovespeed false)
      (Variables|ElevatorSetup|SetHasMoved? false)
      (else
        (Components|MoveComponentTo _elevatortest (.location (Variables|ElevatorSetup|GetFloor1)) "0, 0, 0" false false _elevatormovespeed false)
        (Variables|ElevatorSetup|SetHasMoved? true)))))

(fn ConstructionScript)