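; DemoPickup is a demo respawning statue pickup that reacts to any overlap but grants nothing.
; Overlapping its box plays an explosion and sound, toggles the statue's visibility and disables collision.
; After the Respawn delay, it plays respawn effects, toggles visibility back and re-enables collision.
; A PickupBounce timeline maps curves to the statue's bob and spin, though nothing in the graph starts it.
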(event OnComponentBeginOverlap(Box)
  (params (OverlappedComponent :type Primitive%20Component%20Object%20Reference) (OtherActor :type Actor%20Object%20Reference) (OtherComp :type Primitive%20Component%20Object%20Reference) (OtherBodyIndex :type Integer) (bFromSweep :type Boolean) (SweepResult :type Hit%20Result%20Structure%20%28by%20ref%29))
  (bind _returnvalue (Transformation|GetActorLocation))
  (bind _sm_statue (Variables|Default|GetSM_Statue))
  (bind _returnvalue_2 (Transformation|GetWorldLocation _sm_statue))
  (Effects|SpawnEmitteratLocation "/Game/DemoPickup/P_Explosion.P_Explosion" _returnvalue_2)
  (Audio|PlaySoundatLocation "/Game/DemoPickup/razormind_impact_1.razormind_impact_1" _returnvalue_2 "0, 0, 0" 1.0 1.0 0.0 0 0 0)
  (Rendering|ToggleVisibility (Variables|Default|GetSM_Statue) true)
  (Collision|SetCollisionEnabled (Variables|Default|GetBox) "NoCollision")
  (Utilities|FlowControl|Delay (Variables|Default|GetRespawn))
  (Effects|SpawnEmitteratLocation "/Game/DemoPickup/P_Explosion.P_Explosion" _returnvalue)
  (Audio|PlaySoundatLocation "/Game/DemoPickup/razormind_pad_1.razormind_pad_1" _returnvalue "0, 0, 0" 1.0 1.0 0.0 0 0 0)
  (Rendering|ToggleVisibility (Variables|Default|GetSM_Statue) true)
  (Collision|SetCollisionEnabled (Variables|Default|GetBox) "QueryAndPhysics"))

(event EventBeginPlay)

(event EventTick
  (params (DeltaSeconds :type Float%20%28single-precision%29)))

(event EventDestroyed)

(fn ConstructionScript)